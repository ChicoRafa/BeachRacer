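; AI controller that drives a BP_BeachRacerCharacter ball racer along the level's TargetPoint waypoints.
; BeginPlay gathers and sorts the waypoints.
; Until the list runs out, each Tick triggers acceleration, eases rotation toward the current waypoint with RInterpTo and calls a curve-based speed adjustment.
; The same Tick reissues AI MoveTo with an adjusted destination and the waypoint as target actor, advancing the index on success.
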(event EventBeginPlay
  (bind _outactors (Actor|GetAllActorsOfClass "/Script/Engine.TargetPoint"))
  (Variables|Default|SetWayPoints _outactors)
  (Class|AICBallController|SortWayPoints))

(event EventTick
  (params (DeltaSeconds :type Float%20%28single-precision%29))
  (bind _returnvalue (Pawn|GetControlledPawn))
  (if (< (Variables|Default|GetCurrentWaypointIndex) (Utilities|Array|Length (Variables|Default|GetWayPoints)))
    (CallFunction|StartMovingtoNextWaypoint)
    (bind _asbp_beach_racer_character (Utilities|Casting|CastToBP_BeachRacerCharacter _returnvalue))
    (Default|IAAccelerateBall _asbp_beach_racer_character)
    (Transformation|SetActorRotation _asbp_beach_racer_character (Math|Interpolation|RInterpTo (Transformation|GetActorRotation _returnvalue) (Math|Rotator|FindLookatRotation (Transformation|GetActorLocation _returnvalue) (Transformation|GetActorLocation (Utilities|Array|Get(acopy) (Variables|Default|GetWayPoints) (Variables|Default|GetCurrentWaypointIndex)))) (Utilities|Time|GetWorldDeltaSeconds) 1.0))
    (Class|AICBallController|AdjustSpeedBasedonCurve _asbp_beach_racer_character (Math|Rotator|GetRotationXVector (Math|Interpolation|RInterpTo (Transformation|GetActorRotation _returnvalue) (Math|Rotator|FindLookatRotation (Transformation|GetActorLocation _returnvalue) (Transformation|GetActorLocation (Utilities|Array|Get(acopy) (Variables|Default|GetWayPoints) (Variables|Default|GetCurrentWaypointIndex)))) (Utilities|Time|GetWorldDeltaSeconds) 1.0)) (Transformation|GetActorLocation (Utilities|Array|Get(acopy) (Variables|Default|GetWayPoints) (Variables|Default|GetCurrentWaypointIndex))))
    (bind _returnvalue_2 (Class|AICBallController|GetAdjustedDirection (Transformation|GetActorLocation (Utilities|Array|Get(acopy) (Variables|Default|GetWayPoints) (Variables|Default|GetCurrentWaypointIndex)))))
    (AI|AIMoveTo _asbp_beach_racer_character _returnvalue_2 (Utilities|Array|Get(acopy) (Variables|Default|GetWayPoints) (Variables|Default|GetCurrentWaypointIndex)) 5e+01 false
      (:OnSuccess
        (Variables|Default|SetCurrentWaypointIndex (+ 1 (Variables|Default|GetCurrentWaypointIndex)))))))

(fn ConstructionScript)

(fn StartMovingtoNextWaypoint
  (if (not (Variables|Default|GetbIsmoving))
    (Variables|Default|SetbIsmoving true)))