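; Local multiplayer game mode that sets up two player characters on the same machine at BeginPlay.
; It finds PlayerStart actors by matching their display names to P1 and P2, then spawns a separate third-person character class at each.
; The first player controller possesses P1; a second local player is created and its controller possesses P2, with a debug print for each.
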(event EventBeginPlay
  (bind _outactors (Actor|GetAllActorsOfClass "/Script/Engine.PlayerStart"))
  (for _array_element _outactors
    (switch string (Utilities|GetDisplayName _array_element)
      (:P1
        (Variables|Default|SetP1_Start _array_element))
      (:P2
        (Variables|Default|SetP2_Start _array_element))))
  (Utilities|FlowControl|Sequence
    (:then_0
      (bind _returnvalue (Game|SpawnActorfromClass "/Game/ThirdPerson/Blueprints/BP_ThirdPersonCharacter.BP_ThirdPersonCharacter_C" (Transformation|GetActorTransform (Variables|Default|GetP1_Start)) "Undefined" "MultiplyWithRoot" 0 0))
      (bind _output_get (Variables|Default|SetP1_Character _returnvalue))
      (Pawn|Possess (Game|GetPlayerController 0) _output_get)
      (Development|PrintString "P1"))
    (:then_1
      (bind _returnvalue_2 (Game|SpawnActorfromClass "/Game/ThirdPerson/Blueprints/BP_ThirdPersonCharacter_P2.BP_ThirdPersonCharacter_P2_C" (Transformation|GetActorTransform (Variables|Default|GetP2_Start)) "Undefined" "MultiplyWithRoot" 0 0))
      (bind _output_get_2 (Variables|Default|SetP2_Character _returnvalue_2))
      (Class|GameplayStatics|CreatePlayer -1)
      (Pawn|Possess (Game|GetPlayerController 1) _output_get_2)
      (Development|PrintString "P2"))))

(fn ConstructionScript)